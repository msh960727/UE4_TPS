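; BP_CAttachment_Warp is the attachment for the Warp action that controls a decal, likely a warp indicator, based on equip state.
; It hides the Decal component on BeginPlay, shows it on equip and hides it again on unequip.
; Each event calls its parent implementation first, and the Blueprint contains no warp movement logic of its own.
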(event `self.ReceiveBeginPlay`
  (`parent.ReceiveBeginPlay`)
  (`SceneComponent.SetVisibility` (`self.Decal`) false false))

(event `self.OnEquip`
  (`parent.OnEquip`)
  (`SceneComponent.SetVisibility` (`self.Decal`) true false))

(event `self.OnUnequip`
  (`parent.OnUnequip`)
  (`SceneComponent.SetVisibility` (`self.Decal`) false false))

(fn `UserConstructionScript`)